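; BP_Trigger is a miss zone in the VR saber game that catches BP_Object actors the player failed to hit.
; On box overlap, bombs are destroyed without penalty.
; For other objects, it loops over every BP_MissTab, calling MissEvent, adding to the VR pawn's MissScore and destroying the object.
; The score increase sits inside that loop, so it repeats for each tab found.
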(event OnComponentBeginOverlap(Box)
  (params (OverlappedComponent :type Primitive%20Component%20Object%20Reference) (OtherActor :type Actor%20Object%20Reference) (OtherComp :type Primitive%20Component%20Object%20Reference) (OtherBodyIndex :type Integer) (bFromSweep :type Boolean) (SweepResult :type Hit%20Result%20Structure%20%28by%20ref%29))
  ;[1 1 1] If Player missed Object, than when object overlap BP_Trigger, +5 to Miss Score variable and destroy object
  (bind _asobject (Utilities|Casting|CastToBP_Object OtherActor))
  (Variables|Default|SetAs%20Object _asobject)
  (if (Variables|/Game/VRSaberGameTemplate/Blueprints/BP_Object.BP_Object_C|GetBomb _asobject)
    (Actor|DestroyActor (Variables|Default|GetAs%20Object))
    (else
      (bind _outactors (Actor|GetAllActorsOfClass "/Game/VRSaberGameTemplate/Blueprints/BP_MissTab.BP_MissTab_C"))
      (for _array_element _outactors
        (Default|MissEvent _array_element)
        (bind _asbp_vrpawn (Utilities|Casting|CastToBP_VRPawn (Game|Player|GetPlayerPawn 0)))
        (Variables|/Game/VRSaberGameTemplate/Blueprints/BP_VRPawn.BP_VRPawn_C|SetMissScore _asbp_vrpawn (+ (Variables|/Game/VRSaberGameTemplate/Blueprints/BP_VRPawn.BP_VRPawn_C|GetMissScore _asbp_vrpawn) 5.0))
        (Actor|DestroyActor (Variables|Default|GetAs%20Object))))))

(fn ConstructionScript)