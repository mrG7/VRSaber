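; BP_SpeedUp shows a "Speed Up" notice in the VR saber game when the speed changes.
; Its SpeedUpWidgetEvent gets the BP_SpeedUp_Widget from the SpeedUpWidget component, makes the text visible and plays its looping text animation.
; After a short delay it hides the text again, without stopping the animation.
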(event Custom|SpeedUpWidgetEvent
  ;[1 1 1] Set Visibility "Speed Up" text when speed is changed
  (bind _asspeed_up (Utilities|Casting|CastToBP_SpeedUp_Widget (UserInterface|GetUserWidgetObject (Variables|Default|GetSpeedUpWidget))))
  (bind _output_get (Variables|Default|SetAs%20Speed%20UpWidget _asspeed_up))
  (Widget|SetVisibility (Variables|/Game/VRSaberGameTemplate/Widgets/BP_SpeedUp_Widget.BP_SpeedUp_Widget_C|GetSpeedUPText _output_get) "Visible")
  (UserInterface|Animation|PlayAnimation (Variables|Default|GetAs%20Speed%20UpWidget) (Variables|/Game/VRSaberGameTemplate/Widgets/BP_SpeedUp_Widget.BP_SpeedUp_Widget_C|GetTextAnim (Variables|Default|GetAs%20Speed%20UpWidget)) 0.0 0 "Forward" 1.0 false)
  (Utilities|FlowControl|Delay 5.0)
  (Widget|SetVisibility (Variables|/Game/VRSaberGameTemplate/Widgets/BP_SpeedUp_Widget.BP_SpeedUp_Widget_C|GetSpeedUPText (Variables|Default|GetAs%20Speed%20UpWidget)) "Hidden"))

(fn ConstructionScript)