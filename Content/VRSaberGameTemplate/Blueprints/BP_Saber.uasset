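; VR saber actor with a blade that the trigger toggles on and off, along with its collision and a switch sound.
; Blade overlaps play a haptic effect on the holding hand.
; Blocking hits on BP_Object branch by type: normal and repair objects add Score, repair also lowers MissScore, and bombs raise MissScore and notify every BP_MissTab.
; Hit objects hide, play impact or explosion effects, and are destroyed after a delay.
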(event OnComponentHit(BoxBlockCollision)
  (params (HitComponent :type Primitive%20Component%20Object%20Reference) (OtherActor :type Actor%20Object%20Reference) (OtherComp :type Primitive%20Component%20Object%20Reference) (NormalImpulse :type Vector :default "0, 0, 0") (Hit :type Hit%20Result%20Structure%20%28by%20ref%29))
  ;[0.1927 0.1927 0.1927] When a saber blade hit an object, logic is triggered depending on which object was hitting.
  (bind _asbp_object (Utilities|Casting|CastToBP_Object OtherActor))
  (Variables|Default|SetAs%20Object _asbp_object)
  (if (Variables|/Game/VRSaberGameTemplate/Blueprints/BP_Object.BP_Object_C|GetRepair (Variables|Default|GetAs%20Object))
    (Variables|/Game/VRSaberGameTemplate/Blueprints/BP_VRPawn.BP_VRPawn_C|SetScore (Variables|Default|GetAs%20BP%20VRPawn) (+ (Variables|/Game/VRSaberGameTemplate/Blueprints/BP_VRPawn.BP_VRPawn_C|GetScore (Variables|Default|GetAs%20BP%20VRPawn)) 1e+02))
    ;;[1 1 1] If it was Repair Object, than minus five from Miss Score
    (if (>= (Variables|/Game/VRSaberGameTemplate/Blueprints/BP_VRPawn.BP_VRPawn_C|GetMissScore (Variables|Default|GetAs%20BP%20VRPawn)) 5.0)
      (Variables|/Game/VRSaberGameTemplate/Blueprints/BP_VRPawn.BP_VRPawn_C|SetMissScore (Variables|Default|GetAs%20BP%20VRPawn) (- (Variables|/Game/VRSaberGameTemplate/Blueprints/BP_VRPawn.BP_VRPawn_C|GetMissScore (Variables|Default|GetAs%20BP%20VRPawn)) 5.0)))
    ;;;[1 0.04246 0.988] DestroyActorEvent
    (Components|Activation|SetActive (Variables|/Game/VRSaberGameTemplate/Blueprints/BP_Object.BP_Object_C|GetP_Impact (Variables|Default|GetAs%20Object)) true false)
    (Rendering|SetVisibility (Variables|/Game/VRSaberGameTemplate/Blueprints/BP_Object.BP_Object_C|GetStaticMesh (Variables|Default|GetAs%20Object)) false false)
    (Collision|SetCollisionEnabled (Variables|/Game/VRSaberGameTemplate/Blueprints/BP_Object.BP_Object_C|GetStaticMesh (Variables|Default|GetAs%20Object)) "NoCollision")
    (Audio|Components|Audio|Play (Variables|/Game/VRSaberGameTemplate/Blueprints/BP_Object.BP_Object_C|GetRepair_Wav (Variables|Default|GetAs%20Object)) 0.0)
    (Utilities|FlowControl|Delay 2.0)
    (Utilities|IsValid (Variables|Default|GetAs%20Object)
      (:Is%20Valid
        (Actor|DestroyActor (Variables|Default|GetAs%20Object))))
    (elif (Variables|/Game/VRSaberGameTemplate/Blueprints/BP_Object.BP_Object_C|GetBomb (Variables|Default|GetAs%20Object))
      ;;[1 1 1] If Object has Bomb Variable True, than +5 to Miss Score
      (bind _outactors (Actor|GetAllActorsOfClass "/Game/VRSaberGameTemplate/Blueprints/BP_MissTab.BP_MissTab_C"))
      (for _array_element _outactors
        (Default|MissEvent _array_element)
        (Variables|/Game/VRSaberGameTemplate/Blueprints/BP_VRPawn.BP_VRPawn_C|SetMissScore (Variables|Default|GetAs%20BP%20VRPawn) (+ (Variables|/Game/VRSaberGameTemplate/Blueprints/BP_VRPawn.BP_VRPawn_C|GetMissScore (Variables|Default|GetAs%20BP%20VRPawn)) 5.0))
        ;;[0.8934 0.07128 1] DestropyActorEvent
        (Components|Activation|SetActive (Variables|/Game/VRSaberGameTemplate/Blueprints/BP_Object.BP_Object_C|GetP_Explossion (Variables|Default|GetAs%20Object)) true false)
        (Rendering|SetVisibility (Variables|/Game/VRSaberGameTemplate/Blueprints/BP_Object.BP_Object_C|GetStaticMesh (Variables|Default|GetAs%20Object)) false false)
        (Collision|SetCollisionEnabled (Variables|/Game/VRSaberGameTemplate/Blueprints/BP_Object.BP_Object_C|GetStaticMesh (Variables|Default|GetAs%20Object)) "NoCollision")
        (Audio|Components|Audio|Play (Variables|/Game/VRSaberGameTemplate/Blueprints/BP_Object.BP_Object_C|GetExplosion_Cue (Variables|Default|GetAs%20Object)) 0.0)
        (Utilities|FlowControl|Delay 2.0)
        (Utilities|IsValid (Variables|Default|GetAs%20Object)
          (:Is%20Valid
            (Actor|DestroyActor (Variables|Default|GetAs%20Object)))))
      (else
        ;;[1 1 1] If it was simply object, than +100 to Score and Destroy Actor
        (Components|Activation|SetActive (Variables|/Game/VRSaberGameTemplate/Blueprints/BP_Object.BP_Object_C|GetP_Impact (Variables|Default|GetAs%20Object)) true false)
        (Rendering|SetVisibility (Variables|/Game/VRSaberGameTemplate/Blueprints/BP_Object.BP_Object_C|GetStaticMesh (Variables|Default|GetAs%20Object)) false false)
        (Collision|SetCollisionEnabled (Variables|/Game/VRSaberGameTemplate/Blueprints/BP_Object.BP_Object_C|GetStaticMesh (Variables|Default|GetAs%20Object)) "NoCollision")
        (Variables|/Game/VRSaberGameTemplate/Blueprints/BP_VRPawn.BP_VRPawn_C|SetScore (Variables|Default|GetAs%20BP%20VRPawn) (+ (Variables|/Game/VRSaberGameTemplate/Blueprints/BP_VRPawn.BP_VRPawn_C|GetScore (Variables|Default|GetAs%20BP%20VRPawn)) 1e+02))
        (Audio|Components|Audio|Play (Variables|/Game/VRSaberGameTemplate/Blueprints/BP_Object.BP_Object_C|GetHitSound (Variables|Default|GetAs%20Object)) 0.0)
        (Utilities|FlowControl|Delay 2.0)
        (Utilities|IsValid (Variables|Default|GetAs%20Object)
          (:Is%20Valid
            (Actor|DestroyActor (Variables|Default|GetAs%20Object))))))))

(event OnComponentBeginOverlap(BoxOverlapCollision)
  (params (OverlappedComponent :type Primitive%20Component%20Object%20Reference) (OtherActor :type Actor%20Object%20Reference) (OtherComp :type Primitive%20Component%20Object%20Reference) (OtherBodyIndex :type Integer) (bFromSweep :type Boolean) (SweepResult :type Hit%20Result%20Structure%20%28by%20ref%29))
  ;[1 1 1] Haptic Effect
  (Class|PlayerController|PlayHapticEffect (Game|GetPlayerController 0) "/Game/VRSaberGameTemplate/ExampleContent/VRTemplate/Haptics/PistolFireHapticEffect.PistolFireHapticEffect" (select (Utilities|Name|Equal(Name) (Variables|/Script/HeadMountedDisplay.MotionControllerComponent|GetMotionSource (Variables|/Game/VRSaberGameTemplate/ExampleContent/VRTemplate/Blueprints/BP_GrabComponent.BP_GrabComponent_C|GetMotionControllerRef (Variables|Default|GetGrabComponent))) "Left") "Left" "Right") 1.0 false))

(event EventBeginPlay
  ;[1 1 1] EventBeinPlay. Disable Collision. Cast to VR_Pawn
  (Collision|SetCollisionEnabled (Variables|Default|GetBlade) "NoCollision")
  (bind _asbp_vrpawn (Utilities|Casting|CastToBP_VRPawn (Game|Player|GetPlayerPawn 0)))
  (Variables|Default|SetAs%20BP%20VRPawn _asbp_vrpawn))

(event EventTriggerPressed
  (bind _blade (Variables|Default|GetBlade))
  (bind _blade_2 (Variables|Default|GetBlade))
  ;[1 1 1] Switch Saber Blade: visibility and collision
  (Audio|PlaySoundatLocation "/Game/VRSaberGameTemplate/Audio/Wav/Switch_Wav.Switch_Wav" (Transformation|GetActorLocation) "0, 0, 0" 1.0 1.0 0.0 0 0 0 0)
  (Utilities|FlowControl|FlipFlop
    (:A
      (Rendering|SetVisibility _blade true true)
      (Collision|SetCollisionEnabled _blade_2 "QueryAndPhysics")
      (Collision|SetCollisionEnabled (Variables|Default|GetBoxOverlapCollision) "QueryOnly"))
    (:B
      (Rendering|SetVisibility _blade false true)
      (Collision|SetCollisionEnabled _blade_2 "NoCollision"))))

(fn ConstructionScript)