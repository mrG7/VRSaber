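; Spawner for the VR saber game that sends BP_Object targets down three splines and raises difficulty with score.
; Once the pawn's StartGame is set, Tick starts music, background effect and three spawn lanes after a delay.
; Timelines scaled by duration move each object; its destruction triggers the next spawn until MissScore hits the limit.
; A looping timer checks score thresholds, shortening durations and delays, firing BP_SpeedUp widgets and changing Niagara rotation.
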(event Custom|ObjectSpeed
  ;[1 1 1] Event Begin Play. Set timer event, that every 0.1 seconds is check object speed event
  ;[1 1 1] When Score Variable in VR Pawn Reaches a certain mark, speed Object is increase. Duration is the time the object travels along the spline. If initially we set the time to be 3 seconds, then in order to increase the speed of the object, every time the speed increases, we subtract 0.5 from the duration - thus the speed increases. However, when the duration is 0, the object will stop moving. We also reduce the delay time for the destruction of the object, and the delay of the minimum and maximum delay, so that they spawn faster. At the end of each time we increase the speed, we call the appropriate event widget and increase the torque in the Niagara System.
  (if (>= (Variables|/Game/VRSaberGameTemplate/Blueprints/BP_VRPawn.BP_VRPawn_C|GetScore (Variables|Default|GetVRPawn)) 2e+03)
    (Utilities|FlowControl|Sequence
      (:then_0
        (if (>= (Variables|/Game/VRSaberGameTemplate/Blueprints/BP_VRPawn.BP_VRPawn_C|GetScore (Variables|Default|GetVRPawn)) 6e+03)
          (Utilities|FlowControl|Sequence
            (:then_0
              (if (>= (Variables|/Game/VRSaberGameTemplate/Blueprints/BP_VRPawn.BP_VRPawn_C|GetScore (Variables|Default|GetVRPawn)) 1e+04)
                (Utilities|FlowControl|Sequence
                  (:then_0
                    (if (>= (Variables|/Game/VRSaberGameTemplate/Blueprints/BP_VRPawn.BP_VRPawn_C|GetScore (Variables|Default|GetVRPawn)) 1.5e+04)
                      (Utilities|FlowControl|Sequence
                        (:then_0
                          (if (>= (Variables|/Game/VRSaberGameTemplate/Blueprints/BP_VRPawn.BP_VRPawn_C|GetScore (Variables|Default|GetVRPawn)) 2e+04)
                            (Utilities|FlowControl|Sequence
                              (:then_1
                                (Utilities|FlowControl|DoOnce false
                                  (:Completed
                                    (Variables|Default|SetDuration_1 (- (Variables|Default|GetDuration_1) 0.5))
                                    (Variables|Default|SetDuration_2 (- (Variables|Default|GetDuration_2) 0.5))
                                    (Variables|Default|SetDuration_3 (- (Variables|Default|GetDuration_3) 0.5))
                                    (Variables|Default|SetMinDelay 0.2)
                                    (Variables|Default|SetMaxDelay 0.5)
                                    (Variables|Default|SetDelayDestroyObject 1.5)
                                    (Variables|Default|SetSpeedNumber 6.0)
                                    (bind _outactors (Actor|GetAllActorsOfClass "/Game/VRSaberGameTemplate/Blueprints/BP_SpeedUp.BP_SpeedUp_C"))
                                    (for _array_element _outactors
                                      (Default|SpeedUpWidgetEvent _array_element)
                                      (Effects|Components|ParticleSystem|SetVectorParameter (Variables|Default|GetNS_BackGroundEffect) "MeshRotationForce" "-40.000000,-40.000000,-40.000000"))))))))
                        (:then_1
                          (Utilities|FlowControl|DoOnce false
                            (:Completed
                              (Variables|Default|SetDuration_1 (- (Variables|Default|GetDuration_1) 0.5))
                              (Variables|Default|SetDuration_2 (- (Variables|Default|GetDuration_2) 0.5))
                              (Variables|Default|SetDuration_3 (- (Variables|Default|GetDuration_3) 0.5))
                              (Variables|Default|SetMinDelay 0.5)
                              (Variables|Default|SetMaxDelay 1.0)
                              (Variables|Default|SetDelayDestroyObject 2.0)
                              (Variables|Default|SetSpeedNumber 5.0)
                              (bind _outactors_2 (Actor|GetAllActorsOfClass "/Game/VRSaberGameTemplate/Blueprints/BP_SpeedUp.BP_SpeedUp_C"))
                              (for _array_element_2 _outactors_2
                                (Default|SpeedUpWidgetEvent _array_element_2)
                                (Effects|Components|ParticleSystem|SetVectorParameter (Variables|Default|GetNS_BackGroundEffect) "MeshRotationForce" "20.000000,20.000000,20.000000"))))))))
                  (:then_1
                    (Utilities|FlowControl|DoOnce false
                      (:Completed
                        (Variables|Default|SetDuration_1 (- (Variables|Default|GetDuration_1) 0.5))
                        (Variables|Default|SetDuration_2 (- (Variables|Default|GetDuration_2) 0.5))
                        (Variables|Default|SetDuration_3 (- (Variables|Default|GetDuration_3) 0.5))
                        (Variables|Default|SetMinDelay 0.6)
                        (Variables|Default|SetMaxDelay 1.2)
                        (Variables|Default|SetDelayDestroyObject 3.0)
                        (Variables|Default|SetSpeedNumber 4.0)
                        (bind _outactors_3 (Actor|GetAllActorsOfClass "/Game/VRSaberGameTemplate/Blueprints/BP_SpeedUp.BP_SpeedUp_C"))
                        (for _array_element_3 _outactors_3
                          (Default|SpeedUpWidgetEvent _array_element_3)
                          (Effects|Components|ParticleSystem|SetVectorParameter (Variables|Default|GetNS_BackGroundEffect) "MeshRotationForce" "-12.000000,-12.000000,-12.000000"))))))))
            (:then_1
              (Utilities|FlowControl|DoOnce false
                (:Completed
                  (Variables|Default|SetDuration_1 (- (Variables|Default|GetDuration_1) 0.5))
                  (Variables|Default|SetDuration_2 (- (Variables|Default|GetDuration_2) 0.5))
                  (Variables|Default|SetDuration_3 (- (Variables|Default|GetDuration_3) 0.5))
                  (Variables|Default|SetMinDelay 0.7)
                  (Variables|Default|SetMaxDelay 1.5)
                  (Variables|Default|SetDelayDestroyObject 3.5)
                  (Variables|Default|SetSpeedNumber 3.0)
                  (bind _outactors_4 (Actor|GetAllActorsOfClass "/Game/VRSaberGameTemplate/Blueprints/BP_SpeedUp.BP_SpeedUp_C"))
                  (for _array_element_4 _outactors_4
                    (Default|SpeedUpWidgetEvent _array_element_4)
                    (Effects|Components|ParticleSystem|SetVectorParameter (Variables|Default|GetNS_BackGroundEffect) "MeshRotationForce" "6.000000,6.000000,6.000000"))))))))
      (:then_1
        (Utilities|FlowControl|DoOnce false
          (:Completed
            (Variables|Default|SetDuration_1 (- (Variables|Default|GetDuration_1) 0.5))
            (Variables|Default|SetDuration_2 (- (Variables|Default|GetDuration_2) 0.5))
            (Variables|Default|SetDuration_3 (- (Variables|Default|GetDuration_3) 0.5))
            (Variables|Default|SetMinDelay 0.8)
            (Variables|Default|SetMaxDelay 1.7)
            (Variables|Default|SetDelayDestroyObject 4.5)
            (Variables|Default|SetSpeedNumber 2.0)
            (bind _outactors_5 (Actor|GetAllActorsOfClass "/Game/VRSaberGameTemplate/Blueprints/BP_SpeedUp.BP_SpeedUp_C"))
            (for _array_element_5 _outactors_5
              (Default|SpeedUpWidgetEvent _array_element_5)
              (Effects|Components|ParticleSystem|SetVectorParameter (Variables|Default|GetNS_BackGroundEffect) "MeshRotationForce" "3.000000,3.000000,3.000000"))))))))

(event Custom|EventDestroyedObject
  (params (DestroyedActor :type Actor%20Object%20Reference))
  ;[1 1 1] Spawn Object 1 script
  (if (not (>= (Variables|/Game/VRSaberGameTemplate/Blueprints/BP_VRPawn.BP_VRPawn_C|GetMissScore (Variables|Default|GetVRPawn)) 1e+02))
    (CallFunction|SpawnObject1)))

(event Custom|SpawnObject1
  ;[1 1 1] Spawn Object 1 script
  (Utilities|FlowControl|Delay (Math|Random|RandomFloatinRange (Variables|Default|GetMinDelay) (Variables|Default|GetMaxDelay)))
  (bind _returnvalue (Game|SpawnActorfromClass "/Game/VRSaberGameTemplate/Blueprints/BP_Object.BP_Object_C" (Transformation|GetWorldTransform (Variables|Default|GetArrow)) "Undefined" 0 0))
  (bind _output_get (Variables|Default|SetObject_1 _returnvalue))
  (Transformation|SetWorldScale3D (Variables|/Script/Engine.Actor|GetRootComponent _output_get) "0.500000,0.500000,0.500000")
  (Components|Timeline|SetPlayRate (Variables|Default|GetTimeline_0) (/ 1.0 (Variables|Default|GetDuration_1)))
  (Components|Timeline|SetNewTime (Variables|Default|GetTimeline_0) (Variables|Default|GetNew%20Time_1))
  (bind _alpha (Timeline|Timeline_0 Play)
    (:Update
      (Variables|Default|SetAlpha_1 _alpha)
      (Utilities|IsValid (Variables|Default|GetObject_1)
        (:Is%20Valid
          (Transformation|SetActorLocationAndRotation (Variables|Default|GetObject_1) (Spline|GetLocationatDistanceAlongSpline (Variables|Default|GetSpline) (Math|Float|Lerp 0.0 (Spline|GetSplineLength (Variables|Default|GetSpline)) (Variables|Default|GetAlpha_1)) "World") (Spline|GetRotationatDistanceAlongSpline (Variables|Default|GetSpline) (Math|Float|Lerp 0.0 (Spline|GetSplineLength (Variables|Default|GetSpline)) (Variables|Default|GetAlpha_1)) "World") true true)
          (Utilities|IsValid (Variables|Default|GetObject_1)
            (:Is%20Valid
              (Game|BindEventtoOnDestroyed (Variables|Default|GetObject_1) (delegate Custom|EventDestroyedObject)))))))))

(event Custom|SpawnObject3
  ;[1 1 1] Spawn Object 3 Script. As in the first and second cases, the object at the end of the path is destroyed, regardless of whether it was broken, and then a check follows whether the game is over, and if not, the script is repeated. Also applies to Spawn Object 1 and 2.
  (Utilities|FlowControl|Delay (Math|Random|RandomFloatinRange (Variables|Default|GetMaxDelay) (Variables|Default|GetMaxDelay)))
  (bind _returnvalue (Game|SpawnActorfromClass "/Game/VRSaberGameTemplate/Blueprints/BP_Object.BP_Object_C" (Transformation|GetWorldTransform (Variables|Default|GetArrow2)) "Undefined" 0 0))
  (bind _output_get (Variables|Default|SetObject_3 _returnvalue))
  (Transformation|SetWorldScale3D (Variables|/Script/Engine.Actor|GetRootComponent _output_get) "0.500000,0.500000,0.500000")
  (Components|Timeline|SetPlayRate (Variables|Default|GetTimeline_2) (/ 1.0 (Variables|Default|GetDuration_3)))
  (Components|Timeline|SetNewTime (Variables|Default|GetTimeline_2) (Variables|Default|GetNew%20Time_3))
  (bind _alpha (Timeline|Timeline_2 Play)
    (:Update
      (Variables|Default|SetAlpha_3 _alpha)
      (Utilities|IsValid (Variables|Default|GetObject_3)
        (:Is%20Valid
          (Transformation|SetActorLocationAndRotation (Variables|Default|GetObject_3) (Spline|GetLocationatDistanceAlongSpline (Variables|Default|GetSpline2) (Math|Float|Lerp 0.0 (Spline|GetSplineLength (Variables|Default|GetSpline2)) (Variables|Default|GetAlpha_3)) "World") (Spline|GetRotationatDistanceAlongSpline (Variables|Default|GetSpline2) (Math|Float|Lerp 0.0 (Spline|GetSplineLength (Variables|Default|GetSpline2)) (Variables|Default|GetAlpha_3)) "World") true true)
          (Utilities|IsValid (Variables|Default|GetObject_3)
            (:Is%20Valid
              (Game|BindEventtoOnDestroyed (Variables|Default|GetObject_3) (delegate Custom|EventOnDestroyedObject3)))))))))

(event Custom|EventDestoyedObject2
  (params (DestroyedActor :type Actor%20Object%20Reference))
  ;[1 1 1] Spawn Object 2 Script
  (if (not (>= (Variables|/Game/VRSaberGameTemplate/Blueprints/BP_VRPawn.BP_VRPawn_C|GetMissScore (Variables|Default|GetVRPawn)) 1e+02))
    (CallFunction|SpawnObject2)))

(event Custom|EventOnDestroyedObject3
  (params (DestroyedActor :type Actor%20Object%20Reference))
  ;[1 1 1] Spawn Object 3 Script. As in the first and second cases, the object at the end of the path is destroyed, regardless of whether it was broken, and then a check follows whether the game is over, and if not, the script is repeated. Also applies to Spawn Object 1 and 2.
  (if (not (>= (Variables|/Game/VRSaberGameTemplate/Blueprints/BP_VRPawn.BP_VRPawn_C|GetMissScore (Variables|Default|GetVRPawn)) 1e+02))
    (CallFunction|SpawnObject3)))

(event Custom|SpawnObject2
  ;[1 1 1] Spawn Object 2 Script
  (Utilities|FlowControl|Delay (Math|Random|RandomFloatinRange (Variables|Default|GetMinDelay) (Variables|Default|GetMaxDelay)))
  (bind _returnvalue (Game|SpawnActorfromClass "/Game/VRSaberGameTemplate/Blueprints/BP_Object.BP_Object_C" (Transformation|GetWorldTransform (Variables|Default|GetArrow1)) "Undefined" 0 0))
  (bind _output_get (Variables|Default|SetObject_2 _returnvalue))
  (Transformation|SetWorldScale3D (Variables|/Script/Engine.Actor|GetRootComponent _output_get) "0.500000,0.500000,0.500000")
  (Components|Timeline|SetPlayRate (Variables|Default|GetTimeline_1) (/ 1.0 (Variables|Default|GetDuration_2)))
  (Components|Timeline|SetNewTime (Variables|Default|GetTimeline_1) (Variables|Default|GetNew%20Time_2))
  (bind _alpha (Timeline|Timeline_1 Play)
    (:Update
      (Variables|Default|SetAlpha_2 _alpha)
      (Utilities|IsValid (Variables|Default|GetObject_2)
        (:Is%20Valid
          (Transformation|SetActorLocationAndRotation (Variables|Default|GetObject_2) (Spline|GetLocationatDistanceAlongSpline (Variables|Default|GetSpline1) (Math|Float|Lerp 0.0 (Spline|GetSplineLength (Variables|Default|GetSpline1)) (Variables|Default|GetAlpha_2)) "World") (Spline|GetRotationatDistanceAlongSpline (Variables|Default|GetSpline1) (Math|Float|Lerp 0.0 (Spline|GetSplineLength (Variables|Default|GetSpline1)) (Variables|Default|GetAlpha_2)) "World") true true)
          (Utilities|IsValid (Variables|Default|GetObject_2)
            (:Is%20Valid
              (Game|BindEventtoOnDestroyed (Variables|Default|GetObject_2) (delegate Custom|EventDestoyedObject2)))))))))

(event EventBeginPlay
  ;[1 1 1] Event Begin Play. Set timer event, that every 0.1 seconds is check object speed event
  (bind _asbp_vrpawn (Utilities|Casting|CastToBP_VRPawn (Game|Player|GetPlayerPawn 0)))
  (Variables|Default|SetVRPawn _asbp_vrpawn)
  (Utilities|Time|SetTimerbyEvent (delegate Custom|ObjectSpeed) 0.1 true))

(event EventTick
  (params (DeltaSeconds :type Float%20%28single-precision%29))
  ;[1 1 1] When "Start Game" variable in VR Pawn is true - game is start
  (if (Variables|/Game/VRSaberGameTemplate/Blueprints/BP_VRPawn.BP_VRPawn_C|GetStartGame (Variables|Default|GetVRPawn))
    (Utilities|FlowControl|Delay 3.0)
    (Utilities|FlowControl|Sequence
      (:then_0
        (Utilities|FlowControl|Sequence
          (:then_0
            ;[1 1 1] Start Spawn Objects
            (Utilities|FlowControl|DoOnce false
              (:Completed
                (CallFunction|SpawnObject1))))
          (:then_1
            (Utilities|FlowControl|DoOnce false
              (:Completed
                (CallFunction|SpawnObject2))))
          (:then_2
            (Utilities|FlowControl|DoOnce false
              (:Completed
                (CallFunction|SpawnObject3))))
          (:then_3
            ;[1 1 1] Set Vector Parameter in NS_Background (start rotating effect)
            (Utilities|FlowControl|DoOnce false
              (:Completed
                (Effects|Components|ParticleSystem|SetVectorParameter (Variables|Default|GetNS_BackGroundEffect) "MeshRotationForce" "1.000000,1.000000,1.000000"))))))
      (:then_1
        ;[1 1 1] Play Music
        (Utilities|FlowControl|DoOnce false
          (:Completed
            (Audio|Components|Audio|Play (Variables|Default|GetMusic) 0.0)))))))

(fn ConstructionScript)