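; BP_Object is a spawned target in the VR saber game that becomes a normal shape, bomb or repair object at random.
; BeginPlay schedules self-destruction using the delay read from BP_ObjectSpawner.
; It also sets the mesh and Bomb/Repair flags, with a saber-blade material marking repair cubes.
; Each nested branch rolls a fresh random number, so odds are uneven and defaults can remain.
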(event EventBeginPlay
  (bind _staticmesh (Variables|Default|GetStaticMesh))
  ;[1 1 1] Event Begin Play. Destroy actor after delay (if not broken by saber).
  (Utilities|FlowControl|Sequence
    (:then_0
      (bind _outactors (Actor|GetAllActorsOfClass "/Game/VRSaberGameTemplate/Blueprints/BP_ObjectSpawner.BP_ObjectSpawner_C"))
      (for _array_element _outactors
        (Utilities|FlowControl|Delay (Variables|/Game/VRSaberGameTemplate/Blueprints/BP_ObjectSpawner.BP_ObjectSpawner_C|GetDelayDestroyObject _array_element))
        (Actor|DestroyActor)))
    (:then_1
      ;[1 1 1] Set random static mesh and properties  an object
      (if (== (Math|Random|RandomIntegerinRange 0 5) 0)
        (Components|StaticMesh|SetStaticMesh (Variables|Default|GetStaticMesh) "/Game/VRSaberGameTemplate/ExampleContent/StaticMeshes/SM_Cube_01.SM_Cube_01")
        (Variables|Default|SetBomb false)
        (Variables|Default|SetRepair false)
        (elif (== (Math|Random|RandomIntegerinRange 0 5) 1)
          (Components|StaticMesh|SetStaticMesh (Variables|Default|GetStaticMesh) "/Game/VRSaberGameTemplate/ExampleContent/StaticMeshes/SM_Pyramid_01.SM_Pyramid_01")
          (Variables|Default|SetBomb false)
          (Variables|Default|SetRepair false)
          (elif (== (Math|Random|RandomIntegerinRange 0 5) 2)
            (Components|StaticMesh|SetStaticMesh (Variables|Default|GetStaticMesh) "/Game/VRSaberGameTemplate/ExampleContent/StaticMeshes/SM_Cube_03.SM_Cube_03")
            (Variables|Default|SetBomb false)
            (Variables|Default|SetRepair false)
            (elif (== (Math|Random|RandomIntegerinRange 0 5) 3)
              (Components|StaticMesh|SetStaticMesh (Variables|Default|GetStaticMesh) "/Game/VRSaberGameTemplate/ExampleContent/StaticMeshes/SM_Cube_01.SM_Cube_01")
              (Variables|Default|SetBomb false)
              (Variables|Default|SetRepair false)
              (elif (== (Math|Random|RandomIntegerinRange 0 5) 4)
                (Components|StaticMesh|SetStaticMesh (Variables|Default|GetStaticMesh) "/Game/VRSaberGameTemplate/ExampleContent/StaticMeshes/SM_Ball_01.SM_Ball_01")
                (Variables|Default|SetBomb true)
                (Variables|Default|SetRepair false)
                (elif (== (Math|Random|RandomIntegerinRange 0 5) 5)
                  (Components|StaticMesh|SetStaticMesh _staticmesh "/Game/VRSaberGameTemplate/ExampleContent/StaticMeshes/SM_Cube_01.SM_Cube_01")
                  (Rendering|Material|SetMaterial _staticmesh 0 "/Game/VRSaberGameTemplate/Materials/M_SaberBladeMaterial.M_SaberBladeMaterial")
                  (Variables|Default|SetRepair true)
                  (Variables|Default|SetBomb false))))))))))

(fn ConstructionScript)