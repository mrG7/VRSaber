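; BP_MissTab is a Blueprint in the VR saber game template that shows "Miss" text when MissEvent is called.
; MissEvent casts the MissWidget component's user widget to BP_Miss_Widget, makes its MissText visible and plays TextAnim with a loop count of zero, which repeats endlessly.
; After a one-second delay it hides the text again without stopping the animation.
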(event Custom|MissEvent
  ;[1 1 1] Set Visibility "Miss" Text when missed
  (bind _asbp_miss_widget (Utilities|Casting|CastToBP_Miss_Widget (UserInterface|GetUserWidgetObject (Variables|Default|GetMissWidget))))
  (bind _output_get (Variables|Default|SetAs%20BP%20Miss%20Widget _asbp_miss_widget))
  (Widget|SetVisibility (Variables|/Game/VRSaberGameTemplate/Widgets/BP_Miss_Widget.BP_Miss_Widget_C|GetMissText _output_get) "Visible")
  (UserInterface|Animation|PlayAnimation (Variables|Default|GetAs%20BP%20Miss%20Widget) (Variables|/Game/VRSaberGameTemplate/Widgets/BP_Miss_Widget.BP_Miss_Widget_C|GetTextAnim (Variables|Default|GetAs%20BP%20Miss%20Widget)) 0.0 0 "Forward" 1.0 false)
  (Utilities|FlowControl|Delay 1.0)
  (Widget|SetVisibility (Variables|/Game/VRSaberGameTemplate/Widgets/BP_Miss_Widget.BP_Miss_Widget_C|GetMissText (Variables|Default|GetAs%20BP%20Miss%20Widget)) "Hidden"))

(fn ConstructionScript)